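; BP_Catapult is a catapult from a homework project (HW_03) that fires through a Shoot event.
; Shoot applies an angular impulse to the spoon mesh, then after a short delay eases its pitch back to zero at constant speed through a next-tick loop.
; Once level, it spawns a fresh BP_Cannonball at the spoon's scene point and resets the DoOnce that blocks repeat shots during the cycle.
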(event `Shoot`
  (bind (_relativerotation_roll _relativerotation_pitch) (`KismetMathLibrary.BreakRotator` (`SceneComponent.RelativeRotation` (`self.SpoonMesh`))))
  ;[1 1 1] Реализуйте механику выстрела
  (`/Engine/EditorBlueprintResources/StandardMacros.DoOnce` false :!label _label
    (:`Completed`
      (`PrimitiveComponent.AddAngularImpulseInDegrees` (`self.SpoonMesh`) (`KismetMathLibrary.MakeVector` 0.0 (`self.Impulse`)) "None" true)
      (`KismetSystemLibrary.Delay` 0.5)
      (`SceneComponent.K2_SetRelativeRotation` (`self.SpoonMesh`) (`KismetMathLibrary.MakeRotator` 0.0 (`KismetMathLibrary.FInterpTo_Constant` _relativerotation_pitch 0.0 (`GameplayStatics.GetWorldDeltaSeconds`) 100.0)) false false :!label _label_2)
      (if (== _relativerotation_pitch 0.0)
        (`|SpawnActorFromClass` "/Game/HW_03/Blueprints/Cannonball/BP_Cannonball.BP_Cannonball_C" (`KismetMathLibrary.MakeTransform` (`SceneComponent.K2_GetComponentLocation` (`self.SpoonScene`))) "Undefined" "MultiplyWithRoot" null null)
        (goto _label :!via `Reset`)
        (else
          (`KismetSystemLibrary.DelayUntilNextTick`)
          (goto _label_2))))))

(fn `UserConstructionScript`)