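; BP_Cannonball is a cannonball actor that explodes when it strikes something at speed.
; Its Sphere component's hit event ignores actors tagged "Catapult" and impacts where the ball's velocity is at or below a speed threshold.
; A qualifying hit spawns an explosion particle effect and sound at the ball's location, then destroys the ball without applying damage.
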(event `self.Sphere.OnComponentHit`
  (params (HitComponent :type "PrimitiveComponent Object Reference") (OtherActor :type "Actor Object Reference") (OtherComp :type "PrimitiveComponent Object Reference") (NormalImpulse :type "Vector Structure") (Hit :type "HitResult Structure (by ref)"))
  (bind _returnvalue (`self.K2_GetActorLocation`))
  (`/Engine/EditorBlueprintResources/StandardMacros.IsValid` OtherActor
    (:`Is Valid`
      (if (and (not (`self.ActorHasTag` OtherActor "Catapult")) (> (`KismetMathLibrary.VSize` (`self.GetVelocity`)) 200.0))
        (`GameplayStatics.SpawnEmitterAtLocation` "/Game/StarterContent/Particles/P_Explosion.P_Explosion" _returnvalue)
        (`GameplayStatics.PlaySoundAtLocation` "/Game/StarterContent/Audio/Explosion_Cue.Explosion_Cue" _returnvalue (struct) 1.0 1.0 0.0 null null null null)
        (`self.K2_DestroyActor`)))))

(fn `UserConstructionScript`)